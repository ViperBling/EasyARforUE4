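; BP_ImageTrackerTest is a test Blueprint that runs image tracking with a camera background on screen.
; On BeginPlay it adds a UI_CameraBack widget to the viewport, then configures and initializes ImageTrackers with an image collection, dimensions and output render target.
; It passes the tracker's camera background and render target to the widget before starting tracking.
; Tick drives the tracker every frame.
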(event EventBeginPlay
  (bind _imagetrackers (Variables|Default|GetImageTrackers))
  (bind _returnvalue (UserInterface|CreateWidget "/EasyARforUE4/UI_CameraBack.UI_CameraBack_C" (Game|GetPlayerController 0)))
  (bind _output_get (Variables|Default|SetCamera%20Back _returnvalue))
  (UserInterface|Viewport|AddtoViewport _output_get 0)
  (Variables|/Script/EasyARforUE4.ImageTrackers|SetImageCollection _imagetrackers (Variables|Default|GetImage%20Collection))
  (Variables|/Script/EasyARforUE4.ImageTrackers|SetWidth _imagetrackers (Variables|Default|GetWidth))
  (Variables|/Script/EasyARforUE4.ImageTrackers|SetHeight _imagetrackers (Variables|Default|GetHeight))
  (Class|ImageTrackers|Initialize _imagetrackers)
  (bind _output_get_2 (Variables|/Script/EasyARforUE4.ImageTrackers|SetOutRT _imagetrackers (Variables|Default|GetOut%20RT)))
  (Default|GetBrush0 _output_get (Variables|/Script/EasyARforUE4.ImageTrackers|GetCameraBackground _imagetrackers) _output_get_2)
  (Class|ImageTrackers|Start _imagetrackers))

(event EventTick
  (params (DeltaSeconds :type Float%20%28single-precision%29))
  (Class|ImageTrackers|CallEveryFrame (Variables|Default|GetImageTrackers) DeltaSeconds))

(fn ConstructionScript)