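; Test Blueprint for device camera capture, apparently on Android, that starts a webcam feed when play begins.
; BeginPlay enumerates webcam capture devices filtered to rear-facing, prints the first device's URL and opens it on the CameraMedia player, without checking that a device was found.
; Unconnected leftover nodes would create a UI_MeidaTexture widget and apply the M_CameraTexture material to an image, but never run.
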(event EventBeginPlay
  (bind _outdevices (Class|MediaBlueprintFunctionLibrary|EnumerateWebcamCaptureDevices (|BitmaskLiteral 4)))
  (Development|PrintString (.Url (Utilities|Struct|BreakMediaCaptureDevice (Utilities|Array|Get(acopy) _outdevices))))
  (Class|MediaPlayer|OpenUrl (Variables|Default|GetCameraMedia) (.Url (Utilities|Struct|BreakMediaCaptureDevice (Utilities|Array|Get(acopy) _outdevices)))))

(event Collision|EventActorBeginOverlap
  (params (OtherActor :type Actor%20Object%20Reference)))

(event EventTick
  (params (DeltaSeconds :type Float%20%28single-precision%29)))

(fn ConstructionScript)